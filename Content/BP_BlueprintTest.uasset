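; BP_BlueprintTest is an actor Blueprint that appears to be a scratch test of basic graph nodes, with no clear gameplay role.
; BeginPlay resets relative location and rotation behind a constant-true branch, then runs an empty loop.
; A function holds an unreachable tick toggle and returns fixed booleans.
; A macro sets scale from its input, calls SimpleMoveToActor and always exits through Confirmed, leaving DataLoss unreachable.
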(event `self.ReceiveBeginPlay`
  (if true
    (`self.K2_SetActorRelativeLocation` (0.0 0.0 0.0))
    (`self.K2_SetActorRotation` (struct))
    (for _ (range 40)
      _)))

(fn `NewFunction_0`
  (params (NewParam :type Boolean) (NewParam1 :type Boolean))
  (returns (NewParam2 :type Boolean) (NewParam3 :type Boolean))
  (if (not true)
    (`self.SetActorTickEnabled` NewParam1))
  (return true false))

(fn `UserConstructionScript`)